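; BP_TelsaAlive is the Telsa NPC, a behavior-tree-driven enemy whose appearance shifts from real to ghost as the player gets close.
; A looping timer maps player distance into the MPC_GhostAppearance collection.
; Overlapping BP_Candles forces full ghost, plays a back-walk montage, then flags the hit on the blackboard.
; It also handles talk and discovery voices via subtitles or async-loaded sound fallbacks, plus damage screams and delayed destruction on death.
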(event OnComponentBeginOverlap(CapsuleComponent)
  (params (OverlappedComponent :type Primitive%20Component%20Object%20Reference) (OtherActor :type Actor%20Object%20Reference) (OtherComp :type Primitive%20Component%20Object%20Reference) (OtherBodyIndex :type Integer) (bFromSweep :type Boolean) (SweepResult :type Hit%20Result%20Structure%20%28by%20ref%29))
  (if (Utilities|Enum|Equal(Enum) (Utilities|GetDisplayName OtherActor) "BP_Candles")
    (Utilities|FlowControl|DoOnce false :!label _label
      (:Completed
        (Utilities|Time|ClearandInvalidateTimerbyHandle (Variables|Default|GetTurnTH))
        (Rendering|Material|SetScalarParameterValue "/Game/Characters/Telsa_Ghost/Materials/MPC_GhostAppearance.MPC_GhostAppearance" "RealToGhost" 1.0 :!class /Script/Engine.KismetMaterialLibrary)
        (Animation|Montage|PlayMontage (Variables|Character|GetMesh) "/Game/Characters/Telsa_Alive/Anim/HitCandle/telsa_Move_Walk01_Back_Montage.telsa_Move_Walk01_Back_Montage"
          (:OnCompleted
            (CallFunction|InformHittoBT true))
          (:OnInterrupted
            _))
        (Class|IEnemies|ISetMovementSpeed self false)
        (if (not (Utilities|Time|IsTimerActivebyHandle (Variables|Default|GetTurnTH)))
          (bind _returnvalue (Utilities|Time|SetTimerbyEvent (delegate Custom|TurnOut) 0.05 true))
          (Variables|Default|SetTurnTH _returnvalue)
          (goto _label Reset)
          (else
            (goto _label Reset)))))))

(event Custom|TurnOut
  (bind _returnvalue (Class|HelperFunctions|GetActivePlayerCharacter))
  (bind _returnvalue_2 (Transformation|GetDistanceTo _returnvalue))
  ;[0.05725 1 0] Ghost effect
  (Utilities|IsValid _returnvalue
    (:Is%20Valid
      (if (< _returnvalue_2 3e+02)
        (Rendering|Material|SetScalarParameterValue "/Game/Characters/Telsa_Ghost/Materials/MPC_GhostAppearance.MPC_GhostAppearance" "RealToGhost" (Math|Float|MapRangeClamped _returnvalue_2 3e+02 2e+02 0.0 1.0) :!class /Script/Engine.KismetMaterialLibrary)
        (else
          (Rendering|Material|SetScalarParameterValue "/Game/Characters/Telsa_Ghost/Materials/MPC_GhostAppearance.MPC_GhostAppearance" "RealToGhost" 0.0 :!class /Script/Engine.KismetMaterialLibrary))))
    (:Is%20Not%20Valid
      (Utilities|Time|ClearandInvalidateTimerbyHandle (Variables|Default|GetTurnTH)))))

(event Custom|CreateFloatThingsComp
  ;[0.9948 0.6612 0] FloatThings comp
  (bind _returnvalue (Game|AddComponentbyClass "/Game/Blueprints/Components/BPAC_FloatThings.BPAC_FloatThings_C"))
  (Variables|Default|SetFloatThingsComp _returnvalue)
  (Components|Activation|SetAutoActivate _returnvalue true)
  (bind _returnvalue_2 (Game|AddComponentbyClass "/Script/Engine.BoxComponent" false))
  (bind _output_get (Variables|Default|SetBoxFloatThings _returnvalue_2))
  (Components|Box|SetBoxExtent _output_get "105.107864,168.891510,61.051826" true)
  (Collision|SetCollisionEnabled _output_get "QueryAndPhysics")
  (Collision|SetCollisionProfileName _output_get "OverlapAllDynamic" true :!class /Script/Engine.PrimitiveComponent))

(event EventBeginPlay
  (|CallParentFunction)
  ;[0.05725 1 0] Ghost effect
  (bind _returnvalue (Utilities|Time|SetTimerbyEvent (delegate Custom|TurnOut) 0.05 true))
  (Variables|Default|SetTurnTH _returnvalue))

(event EventIReceiveDamage
  (params (HurtPoint :type Integer))
  ;[1 1 1] Daño
  (if (not (Variables|Default|GetbIsDead))
    (Audio|SpawnSoundAttached "/Game/Audio/SFX/SFX_GhostScream.SFX_GhostScream" (Variables|Character|GetMesh) "None" (Transformation|GetActorLocation) (Transformation|GetActorRotation) "SnapToTarget" true 1.0 (Math|Random|RandomFloatinRange 0.8 1.2) 0.0 "/Game/Audio/Attenuations/SA_IAAttenuation.SA_IAAttenuation" 0)
    (bind _output_get (Variables|Default|SetCurrentHealth (- (Variables|Default|GetCurrentHealth) HurtPoint)))
    (bind _output_get_2 (Variables|Default|SetbIsDead (<= _output_get 0)))
    ;;[1 1 1] para cuando reciba daño
    (if _output_get_2
      (Class|SpectralCharacter|TurnLogic false)
      (Utilities|FlowControl|Delay 5.0)
      (Actor|DestroyActor))))

(event EventDestroyed
  (Utilities|Time|ClearandInvalidateTimerbyHandle (Variables|Default|GetTurnTH)))

(event EventISetAttack
  (|CallParentFunction))

(event EventIFoundTarget
  (bind _returnvalue (Class|HelperFunctions|GetActivePlayerController))
  (bind _discoveredsubtitles (Variables|Default|GetDiscoveredSubtitles))
  (bind _returnvalue_2 (Actor|GetComponentbyClass _returnvalue "/Game/Blueprints/Components/BPAC_Subtitles.BPAC_Subtitles_C"))
  ;[0.5 0 0] New Subtitles when close Y SI EL PLAYER CONTROLLER ES NULL? Y SI el subtitulo es invalido?
  (Utilities|IsValid _returnvalue_2
    (:Is%20Valid
      (if (Utilities|Array|IsValidIndex _discoveredsubtitles)
        (Default|PlaySubtitleAttachCharacter _returnvalue_2 (Variables|Character|GetMesh) (Transformation|GetActorLocation) (Transformation|GetActorRotation) "/Game/Audio/Attenuations/SA_IAAttenuation.SA_IAAttenuation" (Utilities|Array|Get(acopy) _discoveredsubtitles (Math|Random|RandomIntegerinRange 0 (- (Utilities|Array|Length _discoveredsubtitles) 1))))
        (Development|PrintString "SUBTITLE")))
    (:Is%20Not%20Valid
      ;[0.9948 0.6612 0] Found target sound.
      (bind _playingsound (Variables|Default|GetPlayingSound)
        (:then
          (Audio|Components|Audio|Stop _playingsound)
          (Utilities|FlowControl|Delay 0.5))
        (:else
          _))
      (bind _object (Utilities|AsyncLoadAsset (Utilities|Select :Index (Math|Random|RandomIntegerinRange 0 2) :Option%200 "/Game/Audio/Voices/Telsa/T_AlanDiscovered19.T_AlanDiscovered19" :Option%201 "/Game/Audio/Voices/Telsa/T_AlanDiscovered20.T_AlanDiscovered20" :Option%202 "/Game/Audio/Voices/Telsa/T_AlanDiscovered21.T_AlanDiscovered21"))
        (:Completed
          (bind _assound_base (Utilities|Casting|CastToSoundBase _object))
          (Audio|SpawnSoundAttached _assound_base (Variables|Character|GetMesh) "None" (Transformation|GetActorLocation) (Transformation|GetActorRotation) "KeepRelativeOffset" false 1.0 1.0 0.0 0 0))))))

(event EventISetMovementSpeed
  (params (bAlertedMovementSpeed :type Boolean))
  (|CallParentFunction bAlertedMovementSpeed))

(event EventIInterruptCinematic
  (|CallParentFunction))

(event EventICallWalkingAudio
  (params (bNewOn :type Boolean))
  (bind _returnvalue (Class|HelperFunctions|GetActivePlayerController))
  (bind _returnvalue_2 (Math|Random|RandomInteger 9999))
  (bind _talkingaudio (Variables|Default|GetTalkingAudio))
  (bind _talkingaudio_2 (Variables|Default|GetTalkingAudio))
  (bind _talkingsubtitles (Variables|Default|GetTalkingSubtitles))
  (bind _returnvalue_3 (Utilities|Array|Length _talkingaudio))
  (bind _returnvalue_4 (Utilities|Array|Length _talkingsubtitles))
  (bind _returnvalue_5 (Actor|GetComponentbyClass _returnvalue "/Game/Blueprints/Components/BPAC_Subtitles.BPAC_Subtitles_C"))
  (bind _returnvalue_6 (Math|Random|MakeRandomStream _returnvalue_2))
  (bind _returnvalue_7 (- _returnvalue_3 1))
  (bind _returnvalue_8 (- _returnvalue_4 1))
  (bind _returnvalue_9 (Class|KismetMathLibrary|RandomIntegerfromStream _returnvalue_7 _returnvalue_6))
  (bind _returnvalue_10 (Math|Random|RandomIntegerinRange 0 _returnvalue_8))
  (bind _output (Utilities|Array|Get(acopy) _talkingaudio_2 _returnvalue_9))
  ;[1 0.5895 0.1834] New Subtitles sound
  (Utilities|IsValid _returnvalue_5
    (:Is%20Valid
      (if bNewOn
        (if (Utilities|Array|IsValidIndex _talkingsubtitles)
          (if (!= _returnvalue_10 (Variables|Default|GetPrevAudio))
            (Variables|Default|SetPrevAudio _returnvalue_10)
            (Default|PlaySubtitleAttachCharacter _returnvalue_5 (Variables|Character|GetMesh) (Transformation|GetActorLocation) (Transformation|GetActorRotation) "/Game/Audio/Attenuations/SA_IAAttenuation.SA_IAAttenuation" (Utilities|Array|Get(acopy) (Variables|Default|GetTalkingSubtitles) _returnvalue_10))
            (Development|PrintString "SUBTITLE")))
        (else
          (bind _playingsound (Variables|Default|GetPlayingSound)
            (:then
              (Audio|Components|Audio|Stop _playingsound))
            (:else)))))
    (:Is%20Not%20Valid
      ;[0.9948 0.6612 0] next Step : code
      (if true
        (if (Utilities|Array|IsValidIndex _talkingaudio)
          (Utilities|IsValid (Variables|Default|GetPlayingSound)
            (:Is%20Not%20Valid
              (if (!= _returnvalue_9 (Variables|Default|GetPrevAudio))
                (Variables|Default|SetPrevAudio _returnvalue_9)
                (if (Utilities|IsValidSoftObjectReference _output)
                  (bind _object (Utilities|AsyncLoadAsset _output)
                    (:Completed
                      (bind _assound_base (Utilities|Casting|CastToSoundBase _object))
                      (bind _returnvalue_11 (Audio|SpawnSoundAttached _assound_base (Variables|Character|GetMesh) "None" (Transformation|GetActorLocation) (Transformation|GetActorRotation) "SnapToTarget" true 1.0 1.0 0.0 "/Game/Audio/Attenuations/SA_IAAttenuation.SA_IAAttenuation" 0))
                      (Variables|Default|SetPlayingSound _returnvalue_11))))))))
        (else
          (bind _playingsound_2 (Variables|Default|GetPlayingSound)
            (:then
              (Audio|Components|Audio|Stop _playingsound_2))
            (:else)))))))

(fn ConstructionScript)

(fn InformHittoBT
  (params (BoolValue :type Boolean))
  (bind _returnvalue (Pawn|GetController))
  (bind _returnvalue_2 (AI|GetBlackboard _returnvalue))
  (Utilities|IsValid _returnvalue_2
    (:Is%20Valid
      (AI|Components|Blackboard|SetValueasBool _returnvalue_2 (Variables|Default|GetbHitCandleWall) BoolValue))))

(fn IGetIsDead
  (return (Variables|Default|GetbIsDead)))

(fn IGetBehaviorTreeAsset
  (return (Variables|Default|GetBTToUse)))

(fn IGetIsAttacking
  (bind _returnvalue (|CallParentFunction))
  (return _returnvalue))