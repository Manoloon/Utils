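; Test AI pawn that dies and respawns when its capsule hits an actor implementing IEnemies.
; Every tick it calls IterationRay, whose body is not in this graph.
; On death it stops its brain logic, plays a scream and waits on a retriggerable delay.
; If a TargetPoint exists, it teleports there, is re-possessed by a controller found by class and restarts its logic.
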(event OnComponentHit(CapsuleComponent)
  (params (HitComponent :type Primitive%20Component%20Object%20Reference) (OtherActor :type Actor%20Object%20Reference) (OtherComp :type Primitive%20Component%20Object%20Reference) (NormalImpulse :type Vector :default "0, 0, 0") (Hit :type Hit%20Result%20Structure%20%28by%20ref%29))
  (if (Utilities|DoesObjectImplementInterface OtherActor "/Script/PentaKill_Character.IEnemies")
    (CallFunction|GoingtoDie)))

(event Custom|GoingToDie
  (AI|Logic|StopLogic (Variables|/Script/AIModule.AIController|GetBrainComponent (AI|GetAIController self)) "dead")
  (Audio|SpawnSound2D "/Game/Audio/SFX/ScreamTelsaMonster.ScreamTelsaMonster" 1.0 1.0 0.0 0)
  (Utilities|FlowControl|RetriggerableDelay 2.0)
  (bind _returnvalue (Actor|GetActorOfClass "/Script/Engine.TargetPoint"))
  (Utilities|IsValid _returnvalue
    (:Is%20Valid
      (Transformation|SetActorLocationAndRotation (.location (Transformation|GetActorTransform _returnvalue)) (.rotation (Transformation|GetActorTransform _returnvalue)))
      (bind _returnvalue_2 (Actor|GetActorOfClass (Variables|Default|GetAIControllerClass)))
      (Utilities|FlowControl|Delay 0.2)
      (Pawn|Possess _returnvalue_2 self)
      (Class|BrainComponent|RestartLogic (Variables|/Script/AIModule.AIController|GetBrainComponent (AI|GetAIController self))))))

(event EventBeginPlay)

(event Collision|EventActorBeginOverlap
  (params (OtherActor :type Actor%20Object%20Reference)))

(event EventTick
  (params (DeltaSeconds :type Float%20%28single-precision%29))
  (Class|SpectralCharacter|IterationRay))

(fn ConstructionScript)